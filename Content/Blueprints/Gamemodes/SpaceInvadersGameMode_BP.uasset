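; Space Invaders game mode that runs the start menu and high score screen with a UI-only mouse cursor.
; Loads high scores in the construction script, then BeginPlay creates the start menu and a hidden high score widget.
; Slot widgets are filled with rank, name and run stats, with MaxSlots bounding the row loop.
; Tick polls the high-score-open flag to set widget visibility, without ever hiding the main menu.
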(event EventBeginPlay
  (Variables|Default|SetMusic "/Game/Audio/Starter_Music01.Starter_Music01")
  (Variables|Default|SetPlayerController (Game|GetPlayerController 0))
  (bind _returnvalue (CallFunction|CreateHighScoreWidget))
  (bind _returnvalue_2 (CallFunction|CreateMenuWidget (Variables|Default|GetPlayerController)))
  (Input|SetInputModeUIOnly (Variables|Default|GetPlayerController) 0 "DoNotLock")
  (Variables|/Script/Engine.PlayerController|SetbShowMouseCursor (Variables|Default|GetPlayerController) true))

(event EventTick
  (params (DeltaSeconds :type Float%20%28single-precision%29))
  (CallFunction|ToggleHighScoreandMainMenu (stale EventBeginPlay _returnvalue) (stale EventBeginPlay _returnvalue_2)))

(fn ConstructionScript
  (Class|SpaceInvadersGameMode|LoadHighScore))

(fn CreateHighScoreWidget
  (bind _returnvalue (Class|SpaceInvadersGameMode|GetHighScores))
  (Variables|Default|SetHighScoresRef _returnvalue)
  (bind _returnvalue_2 (UserInterface|CreateWidget "/Game/UI/HighScoreMenu.HighScoreMenu_C" (Variables|Default|GetPlayerController)))
  (Variables|Default|SetHighscoreMenuWidgetRef _returnvalue_2)
  (if (< (Utilities|Array|Length (Variables|Default|GetHighScoresRef)) (Variables|Default|GetMaxSlots))
    (for _index (range (Variables|Default|GetTemp) (- (Utilities|Array|Length (Variables|Default|GetHighScoresRef)) 1))
      (Variables|Default|SetTemp _index)
      (bind _returnvalue_3 (UserInterface|CreateWidget "/Game/UI/HighScoreSlot.HighScoreSlot_C" (Variables|Default|GetPlayerController)))
      (Variables|Default|SetHighScoreSlotRef _returnvalue_3)
      (CallFunction|AddDatatoSlot)
      (Widget|Panel|AddChild (Variables|/Game/UI/HighScoreMenu.HighScoreMenu_C|GetHighScoreVerticalBox (Variables|Default|GetHighscoreMenuWidgetRef)) (Variables|/Game/UI/HighScoreSlot.HighScoreSlot_C|GetPlayerScoreVerticalBox (Variables|Default|GetHighScoreSlotRef))))
    (else
      (for _index_2 (range (Variables|Default|GetTemp) (Variables|Default|GetMaxSlots))
        (Variables|Default|SetTemp _index_2)
        (bind _returnvalue_4 (UserInterface|CreateWidget "/Game/UI/HighScoreSlot.HighScoreSlot_C" (Variables|Default|GetPlayerController)))
        (Variables|Default|SetHighScoreSlotRef _returnvalue_4)
        (CallFunction|AddDatatoSlot)
        (Widget|Panel|AddChild (Variables|/Game/UI/HighScoreMenu.HighScoreMenu_C|GetHighScoreVerticalBox (Variables|Default|GetHighscoreMenuWidgetRef)) (Variables|/Game/UI/HighScoreSlot.HighScoreSlot_C|GetPlayerScoreVerticalBox (Variables|Default|GetHighScoreSlotRef))))))
  (UserInterface|Viewport|AddtoViewport (Variables|Default|GetHighscoreMenuWidgetRef) 0)
  (Widget|SetVisibility (Variables|Default|GetHighscoreMenuWidgetRef) "Hidden")
  (return (Variables|Default|GetHighscoreMenuWidgetRef)))

(fn CreateMenuWidget
  (params (PlayerControllerRef :type Player%20Controller%20Object%20Reference))
  (bind _returnvalue (UserInterface|CreateWidget "/Game/UI/StartMenu.StartMenu_C" PlayerControllerRef))
  (UserInterface|Viewport|AddtoViewport _returnvalue 0)
  (return _returnvalue))

(fn ToggleHighScoreandMainMenu
  (params (HighScoreWidget :type Widget%20Object%20Reference) (MainMenuWidget :type Widget%20Object%20Reference))
  (bind _returnvalue (Class|SpaceInvadersGameMode|GetHighScoreIsOpen))
  (if _returnvalue
    (Widget|SetVisibility HighScoreWidget "Visible")
    (else
      (Widget|SetVisibility HighScoreWidget "Hidden")
      (Widget|SetVisibility MainMenuWidget "Visible"))))

(fn AddDatatoSlot
  (Utilities|FlowControl|Sequence
    (:then_0
      (CallFunction|AddRankNumber))
    (:then_1
      (CallFunction|AddPlayerName))
    (:then_2
      (CallFunction|AddWaveReached))
    (:then_3
      (CallFunction|AddEnemiesKilled))
    (:then_4
      (CallFunction|AddBossesKilled))))

(fn AddRankNumber
  (Variables|/Game/UI/HighScoreSlot.HighScoreSlot_C|SetIndexPointer (Variables|Default|GetHighScoreSlotRef) (+ (Variables|Default|GetTemp) 1)))

(fn AddPlayerName
  (bind _temp (Variables|Default|GetTemp))
  (bind _highscoresref (Variables|Default|GetHighScoresRef))
  (if (Utilities|Array|IsValidIndex _highscoresref _temp)
    (Variables|/Game/UI/HighScoreSlot.HighScoreSlot_C|SetPlayerName (Variables|Default|GetHighScoreSlotRef) (.playername (Utilities|Array|Get(acopy) _highscoresref _temp)))))

(fn AddWaveReached
  (bind _temp (Variables|Default|GetTemp))
  (bind _highscoresref (Variables|Default|GetHighScoresRef))
  (if (Utilities|Array|IsValidIndex _highscoresref _temp)
    (Variables|/Game/UI/HighScoreSlot.HighScoreSlot_C|SetWaveReached (Variables|Default|GetHighScoreSlotRef) (.wavereached (Utilities|Array|Get(acopy) _highscoresref _temp)))))

(fn AddEnemiesKilled
  (bind _temp (Variables|Default|GetTemp))
  (bind _highscoresref (Variables|Default|GetHighScoresRef))
  (if (Utilities|Array|IsValidIndex _highscoresref _temp)
    (Variables|/Game/UI/HighScoreSlot.HighScoreSlot_C|SetEnemiesKilled (Variables|Default|GetHighScoreSlotRef) (.enemieskilled (Utilities|Array|Get(acopy) _highscoresref _temp)))))

(fn AddBossesKilled
  (bind _temp (Variables|Default|GetTemp))
  (bind _highscoresref (Variables|Default|GetHighScoresRef))
  (if (Utilities|Array|IsValidIndex _highscoresref _temp)
    (Variables|/Game/UI/HighScoreSlot.HighScoreSlot_C|SetBossesKilled (Variables|Default|GetHighScoreSlotRef) (.bosseskilled (Utilities|Array|Get(acopy) _highscoresref _temp)))))
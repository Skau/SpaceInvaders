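; Main menu game mode that creates the start menu and a hidden high score screen, with UI-only input and a visible cursor.
; On BeginPlay it fetches the saved high scores and builds slot widgets up to a slot limit.
; Each slot gets rank, player name, wave reached, enemies killed and bosses killed.
; Tick polls the high-score-open flag every frame to swap visibility between the two screens.
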(event EventBeginPlay
  (Variables|Default|SetMusic "/Game/Audio/Starter_Music01.Starter_Music01")
  (Variables|Default|SetPlayerControllerRef (Game|GetPlayerController 0))
  (CallFunction|CreateHighScoreWidget)
  (bind _returnvalue (CallFunction|CreateMenuWidget))
  (Variables|Default|SetMenuWidgetRef _returnvalue)
  (Input|SetInputModeUIOnly (Variables|Default|GetPlayerControllerRef) 0 "DoNotLock")
  (Variables|/Script/Engine.PlayerController|SetbShowMouseCursor (Variables|Default|GetPlayerControllerRef) true))

(event EventTick
  (params (DeltaSeconds :type Float%20%28single-precision%29))
  (CallFunction|ToggleMenuandHighScoreMenu))

(fn ConstructionScript)

(fn CreateHighScoreWidget
  (bind _returnvalue (Class|MainMenuGameMode|GetHighScores))
  (Variables|Default|SetHighscoresRef _returnvalue)
  (bind _returnvalue_2 (UserInterface|CreateWidget "/Game/UI/Highscore/HighScoreMenu.HighScoreMenu_C" (Variables|Default|GetPlayerControllerRef)))
  (Variables|Default|SetHighscoreMenuWidgetRef _returnvalue_2)
  (if (< (Utilities|Array|Length (Variables|Default|GetHighscoresRef)) (Variables|Default|GetMaxSlots))
    (for _index (range (Variables|Default|GetTemp) (- (Utilities|Array|Length (Variables|Default|GetHighscoresRef)) 1))
      (Variables|Default|SetTemp _index)
      (bind _returnvalue_3 (UserInterface|CreateWidget "/Game/UI/Highscore/HighScoreSlot.HighScoreSlot_C" (Variables|Default|GetPlayerControllerRef)))
      (Variables|Default|SetHighScoreSlotRef _returnvalue_3)
      (CallFunction|AddDatatoSlot)
      (Widget|Panel|AddChild (Variables|/Game/UI/Highscore/HighScoreMenu.HighScoreMenu_C|GetHighScoreVerticalBox (Variables|Default|GetHighscoreMenuWidgetRef)) (Variables|/Game/UI/Highscore/HighScoreSlot.HighScoreSlot_C|GetPlayerScoreVerticalBox (Variables|Default|GetHighScoreSlotRef))))
    (else
      (for _index_2 (range (Variables|Default|GetTemp) (Variables|Default|GetMaxSlots))
        (Variables|Default|SetTemp _index_2)
        (bind _returnvalue_4 (UserInterface|CreateWidget "/Game/UI/Highscore/HighScoreSlot.HighScoreSlot_C" (Variables|Default|GetPlayerControllerRef)))
        (Variables|Default|SetHighScoreSlotRef _returnvalue_4)
        (CallFunction|AddDatatoSlot)
        (Widget|Panel|AddChild (Variables|/Game/UI/Highscore/HighScoreMenu.HighScoreMenu_C|GetHighScoreVerticalBox (Variables|Default|GetHighscoreMenuWidgetRef)) (Variables|/Game/UI/Highscore/HighScoreSlot.HighScoreSlot_C|GetPlayerScoreVerticalBox (Variables|Default|GetHighScoreSlotRef))))))
  (UserInterface|Viewport|AddtoViewport (Variables|Default|GetHighscoreMenuWidgetRef) 0)
  (Widget|SetVisibility (Variables|Default|GetHighscoreMenuWidgetRef) "Hidden")
  (return (Variables|Default|GetHighscoreMenuWidgetRef)))

(fn AddDatatoSlot
  (Utilities|FlowControl|Sequence
    (:then_0
      (CallFunction|AddRankNumber))
    (:then_1
      (CallFunction|AddPlayerName))
    (:then_2
      (CallFunction|AddWaveReached))
    (:then_3
      (CallFunction|AddEnemiesKilled))
    (:then_4
      (CallFunction|AddBossesKilled))))

(fn AddRankNumber
  (Variables|/Game/UI/Highscore/HighScoreSlot.HighScoreSlot_C|SetIndexPointer (Variables|Default|GetHighScoreSlotRef) (+ (Variables|Default|GetTemp) 1)))

(fn AddPlayerName
  (bind _temp (Variables|Default|GetTemp))
  (bind _highscoresref (Variables|Default|GetHighscoresRef))
  (if (Utilities|Array|IsValidIndex _highscoresref _temp)
    (Variables|/Game/UI/Highscore/HighScoreSlot.HighScoreSlot_C|SetPlayerName (Variables|Default|GetHighScoreSlotRef) (.playername (Utilities|Array|Get(acopy) _highscoresref _temp)))))

(fn AddWaveReached
  (bind _highscoresref (Variables|Default|GetHighscoresRef))
  (bind _temp (Variables|Default|GetTemp))
  (if (Utilities|Array|IsValidIndex _highscoresref _temp)
    (Variables|/Game/UI/Highscore/HighScoreSlot.HighScoreSlot_C|SetWaveReached (Variables|Default|GetHighScoreSlotRef) (.wavereached (Utilities|Array|Get(acopy) _highscoresref _temp)))))

(fn AddEnemiesKilled
  (bind _temp (Variables|Default|GetTemp))
  (bind _highscoresref (Variables|Default|GetHighscoresRef))
  (if (Utilities|Array|IsValidIndex _highscoresref _temp)
    (Variables|/Game/UI/Highscore/HighScoreSlot.HighScoreSlot_C|SetEnemiesKilled (Variables|Default|GetHighScoreSlotRef) (.enemieskilled (Utilities|Array|Get(acopy) _highscoresref _temp)))))

(fn AddBossesKilled
  (bind _temp (Variables|Default|GetTemp))
  (bind _highscoresref (Variables|Default|GetHighscoresRef))
  (if (Utilities|Array|IsValidIndex _highscoresref _temp)
    (Variables|/Game/UI/Highscore/HighScoreSlot.HighScoreSlot_C|SetBossesKilled (Variables|Default|GetHighScoreSlotRef) (.bosseskilled (Utilities|Array|Get(acopy) _highscoresref _temp)))))

(fn CreateMenuWidget
  (bind _returnvalue (UserInterface|CreateWidget "/Game/UI/StartMenu.StartMenu_C" (Variables|Default|GetPlayerControllerRef)))
  (UserInterface|Viewport|AddtoViewport _returnvalue 0)
  (return _returnvalue))

(fn ToggleMenuandHighScoreMenu
  (bind _returnvalue (Class|MainMenuGameMode|GetHighScoreIsOpen))
  (if _returnvalue
    (Widget|SetVisibility (Variables|Default|GetHighscoreMenuWidgetRef) "Visible")
    (Widget|SetVisibility (Variables|Default|GetMenuWidgetRef) "Hidden")
    (else
      (Widget|SetVisibility (Variables|Default|GetHighscoreMenuWidgetRef) "Hidden")
      (Widget|SetVisibility (Variables|Default|GetMenuWidgetRef) "Visible"))))